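; BP_Enemy_AI is an AI controller that drives BP_Enemy through the BT_Enemy behavior tree.
; On BeginPlay it caches its controlled enemy, starts the tree, stores the player character as CurrentTarget and writes the default state to the AIState blackboard key.
; AIAttack switches that state and updates the blackboard, while Pawn_Attack forwards the attack call to the enemy pawn.
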(event Custom|Pawn_Attack
  ;[1 1 1] Call attack in enemy BP
  (Default|Attack (Variables|Default|GetAs%20BP%20Enemy)))

(event Custom|AIAttack
  (Variables|Default|SetCurrentState "NewEnumerator1")
  (AI|Components|Blackboard|SetValueasEnum (AI|GetBlackboard 0) (Utilities|Name|MakeLiteralName "AIState") (Variables|Default|GetCurrentState)))

(event EventBeginPlay
  (bind _asbp_enemy (Utilities|Casting|CastToBP_Enemy (Pawn|GetControlledPawn)))
  (Variables|Default|SetAs%20BP%20Enemy _asbp_enemy)
  (AI|RunBehaviorTree "/Game/Blueprints/Enemy/BT_Enemy.BT_Enemy")
  (Variables|Default|SetCurrentTarget (Game|GetPlayerCharacter 0))
  ;[1 1 1] Set Default State
  (AI|Components|Blackboard|SetValueasEnum (AI|GetBlackboard 0) (Utilities|Name|MakeLiteralName "AIState") (Variables|Default|GetCurrentState)))

(fn ConstructionScript)