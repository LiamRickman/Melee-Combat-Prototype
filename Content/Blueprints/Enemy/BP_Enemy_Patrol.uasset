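; Patrol enemy character with health, random melee attack montages, hit reactions and death, syncing its alive state to the AI blackboard.
; An overlap sphere shows a camera-facing health bar while the player is near.
; Taking damage feeds player overcharge, updates the widget and plays a reaction montage chosen by damage amount and direction, with DoOnce blocking overlapping hits.
; Death releases the player's target lock, disables mesh collision and destroys the actor after the montage.
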(event OnComponentBeginOverlap(Sphere)
  (params (OverlappedComponent :type Primitive%20Component%20Object%20Reference) (OtherActor :type Actor%20Object%20Reference) (OtherComp :type Primitive%20Component%20Object%20Reference) (OtherBodyIndex :type Integer) (bFromSweep :type Boolean) (SweepResult :type Hit%20Result%20Structure%20%28by%20ref%29))
  ;[1 1 1] Hide/Show Healthbar
  (Utilities|Casting|CastToBP_Player OtherActor)
  (Rendering|SetVisibility (Variables|Default|GetHealthWidget) true false))

(event OnComponentEndOverlap(Sphere)
  (params (OverlappedComponent :type Primitive%20Component%20Object%20Reference) (OtherActor :type Actor%20Object%20Reference) (OtherComp :type Primitive%20Component%20Object%20Reference) (OtherBodyIndex :type Integer))
  ;[1 1 1] Hide/Show Healthbar
  (Utilities|Casting|CastToBP_Player OtherActor)
  (Rendering|SetVisibility (Variables|Default|GetHealthWidget) false false))

(event Custom|Attack
  (Utilities|FlowControl|DoOnce false :!label _label
    (:Completed
      (switch int (Math|Random|RandomIntegerinRange 0 2)
        (:0
          _)
        (:1
          _)
        (:2
          (bind _returnvalue (Animation|PlayAnimMontage "/Game/Animations/Enemy/AM_Attack_L_02.AM_Attack_L_02" 1.0 "None"))
          (Utilities|FlowControl|Delay _returnvalue)
          (goto _label Reset)))
      (bind _returnvalue_2 (Animation|PlayAnimMontage "/Game/Animations/Enemy/AM_Attack_L_01.AM_Attack_L_01" 1.0 "None"))
      (Utilities|FlowControl|Delay _returnvalue_2)
      (goto _label Reset))))

(event Custom|SetDamageDirection
  (params (DamageDirection :type Vector))
  ;[1 1 1] Calculate which direction the damage came from
  (Variables|Default|SetDamageDirection (.y (Math|Transform|InverseTransformLocation (Math|Conversions|ToTransform(Vector) DamageDirection) (Transformation|GetWorldLocation (Variables|Character|GetMesh))))))

(event Custom|KillEnemy
  ;[1 1 1] Kill enemy
  (if (Variables|Default|GetAlive)
    (bind _asbp_player (Utilities|Casting|CastToBP_Player (Game|GetPlayerCharacter 0)))
    (Default|TurnOffTargetLock _asbp_player)
    (Rendering|SetVisibility (Variables|Default|GetHealthWidget) false false)
    (Variables|Default|SetAlive false)
    (Collision|SetCollisionEnabled (Variables|Character|GetMesh) "NoCollision")
    ;;[1 1 1] Updating Behaviour tree
    (AI|Components|Blackboard|SetValueasBool (AI|GetBlackboard (Pawn|GetController)) (Utilities|Name|MakeLiteralName "IsEnemyAlive") (Variables|Default|GetAlive))
    ;;[1 1 1] Play death anim + wait before destroying actor
    (bind _returnvalue (Animation|PlayAnimMontage "/Game/Animations/Enemy/AM_Death_01.AM_Death_01" 1.0 "None"))
    (Utilities|FlowControl|Delay (+ _returnvalue 5.0))
    (Actor|DestroyActor)))

(event EventTick
  (params (DeltaSeconds :type Float%20%28single-precision%29))
  (bind _healthwidget (Variables|Default|GetHealthWidget))
  ;[1 1 1] Update healthbar rotation
  (if (Rendering|IsVisible _healthwidget)
    (Transformation|SetWorldRotation _healthwidget (Math|Rotator|FindLookatRotation (Transformation|GetWorldLocation _healthwidget) (Camera|GetCameraLocation (Game|GetPlayerCameraManager 0))) false false)))

(event EventBeginPlay
  ;[1 1 1] Begin play (setting references, defaults etc)
  (bind _output_get (Variables|Default|SetAlive true))
  (AI|Components|Blackboard|SetValueasBool (AI|GetBlackboard (Pawn|GetController)) (Utilities|Name|MakeLiteralName "IsEnemyAlive") _output_get)
  (bind _aswbp_ai_health (Utilities|Casting|CastToWBP_AI_Health (UserInterface|GetUserWidgetObject (Variables|Default|GetHealthWidget))))
  (Variables|References|SetAs%20WBP%20AI%20Health _aswbp_ai_health)
  (bind _asbp_player (Utilities|Casting|CastToBP_Player (Game|GetPlayerCharacter 0)))
  (Variables|References|SetAs%20BP%20Player _asbp_player))

(event Game|Damage|EventAnyDamage
  (params (Damage :type Float%20%28single-precision%29) (DamageType :type Damage%20Type%20Object%20Reference) (InstigatedBy :type Controller%20Object%20Reference) (DamageCauser :type Actor%20Object%20Reference))
  ;[1 1 1] Take Damage
  (Utilities|FlowControl|DoOnce false :!label _label
    (:Completed
      (bind _output_get (Variables|Default|SetDamageAmount Damage))
      (CallFunction|AddPlayerOvercharge 1e+01)
      ;;[1 1 1] Check if enemy will die
      (if (> (- (Variables|Default|GetHealth) _output_get) 0.0)
        ;;[1 1 1] Adjust health and widget
        (bind _output_get_2 (Variables|Default|SetHealth (- (Variables|Default|GetHealth) (Variables|Default|GetDamageAmount))))
        (Variables|/Game/UI/Blueprints/WBP_AI_Health.WBP_AI_Health_C|SetHealth (Variables|References|GetAs%20WBP%20AI%20Health) _output_get_2)
        (Utilities|PlayDamageAnimation
          (:Output
            (goto _label Reset)))
        (else
          (CallFunction|KillEnemy))))))

(fn ConstructionScript)

(fn AddPlayerOvercharge
  (params (Amount :type Float%20%28single-precision%29))
  (bind _asbp_player (Utilities|Casting|CastToBP_Player (Game|GetPlayerCharacter 0)))
  (LocalVariables|SetLoc_Amount Amount)
  (if (and (< (Variables|/Game/Blueprints/Player/BP_Player.BP_Player_C|GetOverchargeMeter _asbp_player) 1e+02) (Variables|/Game/Blueprints/Player/BP_Player.BP_Player_C|GetCanGainOvercharge _asbp_player))
    (Variables|/Game/Blueprints/Player/BP_Player.BP_Player_C|SetOverchargeMeter _asbp_player (Math|Float|Clamp(Float) (+ (Variables|/Game/Blueprints/Player/BP_Player.BP_Player_C|GetOverchargeMeter _asbp_player) (LocalVariables|GetLoc_Amount)) 0.0 1e+02)))
  (return))