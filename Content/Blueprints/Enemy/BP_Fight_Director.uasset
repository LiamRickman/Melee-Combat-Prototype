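; Fight director that coordinates enemy attacks by ordering the highest-graded enemy's AI to attack on a looping timer.
; Each enemy in EnemyList starts with a random grade, which is rerolled after it attacks.
; Before each pick, grades are multiplied by a forward-vector dot product factor that favors enemies facing opposite to the player's facing, compounding over time.
; A debug widget component attached to each enemy displays its current grade.
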(event Custom|TriggerAttack
  (CallFunction|RecalculateScores)
  (bind _loc_highestgradedenemy1 (CallFunction|FindHighestGrade))
  (bind _asbp_enemy_ai (Utilities|Casting|CastToBP_Enemy_AI (AI|GetAIController _loc_highestgradedenemy1)))
  (Default|AIAttack _asbp_enemy_ai)
  (Utilities|Map|Add (Variables|Default|GetEnemyGrading) _loc_highestgradedenemy1 (Math|Random|RandomFloatinRange 1.0 5.0))
  (CallFunction|UpdateDebugWidgets _loc_highestgradedenemy1))

(event EventBeginPlay
  (for _array_element (Variables|Default|GetEnemyList)
    (CallFunction|AddDebugWidgets _array_element))
  (Utilities|Time|SetTimerbyEvent (delegate Custom|TriggerAttack) 2.0 true))

(fn ConstructionScript)

(fn FindHighestGrade
  (bind _keys (Utilities|Map|Keys (Variables|Default|GetEnemyGrading)))
  (for _array_element _keys
    (if (> (.Value (Utilities|Map|Find (Variables|Default|GetEnemyGrading) _array_element)) (LocalVariables|GetLoc_HighestValue))
      (LocalVariables|SetLoc_HighestValue (.Value (Utilities|Map|Find (Variables|Default|GetEnemyGrading) _array_element)))
      (LocalVariables|SetLoc_HighestGradedEnemy _array_element)))
  (return (LocalVariables|GetLoc_HighestValue) (LocalVariables|GetLoc_HighestGradedEnemy)))

(fn AddDebugWidgets
  (params (EnemyInstance :type BP%20Enemy%20Object%20Reference%20%28by%20ref%29))
  (Utilities|Map|Add (Variables|Default|GetEnemyGrading) EnemyInstance (Math|Random|RandomFloatinRange 1.0 5.0))
  (bind _returnvalue (UserInterface|CreateWidget "/Game/Blueprints/Enemy/WBP_Debug_Enemy_AI.WBP_Debug_Enemy_AI_C" 0 EnemyInstance (.Value (Utilities|Map|Find (Variables|Default|GetEnemyGrading) EnemyInstance))))
  (bind _output_get (LocalVariables|SetLoc_Widget _returnvalue))
  (Utilities|Map|Add (Variables|Default|GetEnemyWidgets) EnemyInstance _output_get)
  (bind _returnvalue_2 (AddComponent|AddWidgetComponent EnemyInstance false))
  (UserInterface|SetWidget _returnvalue_2 (LocalVariables|GetLoc_Widget)))

(fn UpdateDebugWidgets
  (params (EnemyInstance :type BP%20Enemy%20Object%20Reference))
  (Variables|/Game/Blueprints/Enemy/WBP_Debug_Enemy_AI.WBP_Debug_Enemy_AI_C|SetFightingGrade (.Value (Utilities|Map|Find (Variables|Default|GetEnemyWidgets) EnemyInstance)) (.Value (Utilities|Map|Find (Variables|Default|GetEnemyGrading) EnemyInstance))))

(fn RecalculateScores
  (CallFunction|ScorebyPosition))

(fn ScorebyPosition
  (bind _enemygrading (Variables|Default|GetEnemyGrading))
  (for _array_element (Variables|Default|GetEnemyList)
    (Utilities|Map|Add _enemygrading _array_element (* (.Value (Utilities|Map|Find _enemygrading _array_element)) (+ (Math|Float|NormalizetoRange (* (Math|Vector|DotProduct (Transformation|GetActorForwardVector _array_element) (Transformation|GetActorForwardVector (Game|GetPlayerCharacter 0))) -1.0) -1.0 1.0) 0.5)))
    (CallFunction|UpdateDebugWidgets _array_element)))