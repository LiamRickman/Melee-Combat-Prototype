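; Enemy spawner actor that spawns a configurable number of AI pawns of a configurable class at its own location on BeginPlay.
; It enables player input so a debug action can kill every BP_Enemy_Random in the level and spawn a fresh batch.
; Both paths feed a SpawnEnemy event that loops SpawnAIFromClass, with no behavior tree supplied by the callers.
; The delayed repeat-spawn logic is disconnected and never runs.
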(event Custom|SpawnEnemy
  (params (Enemy :type Pawn%20Class%20Reference) (BehaviorTree :type Behavior%20Tree%20Object%20Reference) (Location :type Vector) (No.%20of%20Enemies :type Integer))
  (for _index (range 1 No.%20of%20Enemies)
    (AI|SpawnAIFromClass Enemy BehaviorTree Location "0, 0, 0" false 0)))

(event EventBeginPlay
  (Input|EnableInput (Game|GetPlayerController 0))
  (CallFunction|SpawnEnemy (Variables|Default|GetEnemyType) 0 (Transformation|GetActorLocation) (Variables|Default|GetNumber%20Of%20Enemies)))

(event Input|ActionEvents|InputActionSpawnEnemies(Debug)
  (params (Key :type Key%20Structure :default "None"))
  (:Pressed
    (bind _outactors (Actor|GetAllActorsOfClass "/Game/Blueprints/Enemy/BP_Enemy_Random.BP_Enemy_Random_C"))
    (for _array_element _outactors
      (Default|KillEnemy _array_element))
    (CallFunction|SpawnEnemy (Variables|Default|GetEnemyType) 0 (Transformation|GetActorLocation) (Variables|Default|GetNumber%20Of%20Enemies))))

(fn ConstructionScript)