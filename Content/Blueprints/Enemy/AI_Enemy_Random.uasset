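; AI controller for an enemy that runs the BT_Enemy_Random behavior tree on BeginPlay and feeds player state into its Blackboard.
; Every Tick it reads the player character's Dead flag to set IsPlayerAlive, printing a message if the cast to BP_Player fails.
; AIPerception target updates for BP_Player actors write the stimulus's sensed result to CanSeePlayer, covering both gaining and losing detection.
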(event OnTargetPerceptionUpdated(AIPerception)
  (params (Actor :type Actor%20Object%20Reference) (Stimulus :type AI%20Stimulus%20Structure))
  (Utilities|Casting|CastToBP_Player Actor)
  (AI|Components|Blackboard|SetValueasBool (AI|GetBlackboard 0) (Utilities|Name|MakeLiteralName "CanSeePlayer") (.bSuccessfullySensed (Utilities|Struct|BreakAIStimulus Stimulus))))

(event EventBeginPlay
  (AI|RunBehaviorTree "/Game/Blueprints/Enemy/BT_Enemy_Random.BT_Enemy_Random"))

(event EventTick
  (params (DeltaSeconds :type Float%20%28single-precision%29))
  (Utilities|FlowControl|Sequence
    (:then_0
      (bind _asbp_player (Utilities|Casting|CastToBP_Player (Game|GetPlayerCharacter 0))
        (:then
          (if (Variables|/Game/Blueprints/Player/BP_Player.BP_Player_C|GetDead _asbp_player)
            (AI|Components|Blackboard|SetValueasBool (AI|GetBlackboard 0) (Utilities|Name|MakeLiteralName "IsPlayerAlive") false)
            (else
              (AI|Components|Blackboard|SetValueasBool (AI|GetBlackboard 0) (Utilities|Name|MakeLiteralName "IsPlayerAlive") true))))
        (:CastFailed
          (Development|PrintString "BP_PLayer not found"))))))

(fn ConstructionScript)