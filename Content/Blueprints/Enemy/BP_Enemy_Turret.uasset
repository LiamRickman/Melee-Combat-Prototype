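; BP_Enemy_Turret is an enemy turret that turns toward the player and fires projectiles when its PawnSensing component sees them.
; Each sighting snaps the actor's rotation to face the player, with no interpolation.
; It then spawns a BP_Projectile at ProjectileSpawn and launches it with a velocity-change impulse along the Cube's forward vector.
; A SpawnProjectile flag and a Firerate delay throttle the shots.
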(event OnSeePawn(PawnSensing)
  (params (Pawn :type Pawn%20Object%20Reference))
  (bind _asbp_player (Utilities|Casting|CastToBP_Player Pawn))
  (Utilities|FlowControl|Sequence
    (:then_0
      (Transformation|SetActorRotation (Math|Rotator|FindLookatRotation (Transformation|GetActorLocation) (Transformation|GetActorLocation _asbp_player))))
    (:then_1
      (if (Variables|Default|GetSpawnProjectile)
        (bind _returnvalue (Game|SpawnActorfromClass "/Game/Blueprints/Enemy/BP_Projectile.BP_Projectile_C" (Transformation|GetWorldTransform (Variables|Default|GetProjectileSpawn)) "Undefined" 0 0))
        (Physics|AddImpulse (Variables|/Game/Blueprints/Enemy/BP_Projectile.BP_Projectile_C|GetSphere _returnvalue) (* (Math|Vector|GetForwardVector (Variables|Default|GetCube)) (Variables|Default|GetProjectileForce)) "None" true)
        (Variables|Default|SetSpawnProjectile false)
        (Utilities|FlowControl|Delay (Variables|Default|GetFirerate))
        (Variables|Default|SetSpawnProjectile true)))))

(fn ConstructionScript)