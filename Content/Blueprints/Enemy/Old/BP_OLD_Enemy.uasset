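; Old enemy Blueprint that handles taking damage with directional hit reactions and feeds the player's ultimate charge.
; AnyDamage, gated by a DoOnce, adds charge to BP_Player when allowed, zeroes it past the cap, and lowers Health without any death check.
; A damage threshold and the sideways offset from SetDamageDirection select a light or heavy, left or right montage.
; The gate reopens after the montage's length.
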(event Custom|SetDamageDirection
  (params (DamageDirection :type Vector))
  ;[1 1 1] Calculate which direction the damage came from
  (bind _output_get (Variables|Default|SetDamageDirection (.y (Math|Transform|InverseTransformLocation (Math|Conversions|ToTransform(Vector) DamageDirection) (Transformation|GetWorldLocation (Variables|Character|GetMesh)))))))

(event Game|Damage|EventAnyDamage
  (params (Damage :type Float%20%28single-precision%29) (DamageType :type Damage%20Type%20Object%20Reference) (InstigatedBy :type Controller%20Object%20Reference) (DamageCauser :type Actor%20Object%20Reference))
  (bind _damagedirection (Variables|Default|GetDamageDirection))
  (bind _returnvalue (< _damagedirection 0.0))
  ;[1 1 1] Take Damage/Death
  (Utilities|FlowControl|DoOnce false :!label _label
    (:Completed
      (bind _asbp_player (Utilities|Casting|CastToBP_Player (Game|GetPlayerCharacter 0)))
      (bind _output_get (Variables|Default|SetAs%20BP%20Player _asbp_player))
      (if (and (< (Variables|/Game/Blueprints/Player/BP_Player.BP_Player_C|GetUltimateCharge _output_get) 1e+02) (Variables|/Game/Blueprints/Player/BP_Player.BP_Player_C|GetCanGainUltimate _output_get))
        (bind _output_get_2 (Variables|/Game/Blueprints/Player/BP_Player.BP_Player_C|SetUltimateCharge _output_get (+ (Variables|/Game/Blueprints/Player/BP_Player.BP_Player_C|GetUltimateCharge _output_get) 5e+01))))
      (if (> _output_get_2 1e+02)
        (Variables|/Game/Blueprints/Player/BP_Player.BP_Player_C|SetUltimateCharge _output_get 0.0))
      (bind _output_get_3 (Variables|Default|SetDamageAmount Damage))
      (Variables|EnemyStats|SetHealth (- (Variables|EnemyStats|GetHealth) _output_get_3))
      (if (<= (Variables|Default|GetDamageAmount) 1e+01)
        (if _returnvalue
          (bind _returnvalue_2 (Animation|PlayAnimMontage "/Game/Animations/Enemy/AM_Light_Damage_Left.AM_Light_Damage_Left" 1.0 "None"))
          (Utilities|FlowControl|Delay _returnvalue_2)
          (else
            (bind _returnvalue_3 (Animation|PlayAnimMontage "/Game/Animations/Enemy/AM_Light_Damage_Right.AM_Light_Damage_Right" 1.0 "None"))
            (Utilities|FlowControl|Delay _returnvalue_3)))
        (elif _returnvalue
          (bind _returnvalue_4 (Animation|PlayAnimMontage "/Game/Animations/Enemy/AM_Heavy_Damage_Left.AM_Heavy_Damage_Left" 1.0 "None"))
          (Utilities|FlowControl|Delay _returnvalue_4)
          (else
            (bind _returnvalue_5 (Animation|PlayAnimMontage "/Game/Animations/Enemy/AM_Heavy_Damage_Right.AM_Heavy_Damage_Right" 1.0 "None"))
            (Utilities|FlowControl|Delay _returnvalue_5))))
      (Development|PrintString (Utilities|String|ToString(Float) (stale Custom|SetDamageDirection _output_get)))
      (goto _label Reset))))

(fn ConstructionScript)