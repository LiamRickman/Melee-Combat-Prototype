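; Patrolling enemy character with montage-driven melee attacks, directional hit reactions and death.
; Attack randomly favors the light montage two-to-one; attacks and damage are DoOnce-gated until montages finish.
; Damage updates the health widget, charges the player's ultimate and picks reactions by amount and direction; death toggles lock-on, clears the Blackboard alive flag and destroys the actor after a delay.
; The camera-facing health bar shows while the player overlaps its sphere.
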(event OnComponentBeginOverlap(Sphere)
  (params (OverlappedComponent :type Primitive%20Component%20Object%20Reference) (OtherActor :type Actor%20Object%20Reference) (OtherComp :type Primitive%20Component%20Object%20Reference) (OtherBodyIndex :type Integer) (bFromSweep :type Boolean) (SweepResult :type Hit%20Result%20Structure%20%28by%20ref%29))
  (Utilities|Casting|CastToBP_Player OtherActor)
  (Rendering|SetVisibility (Variables|Default|GetHealthWidget) true false))

(event OnComponentEndOverlap(Sphere)
  (params (OverlappedComponent :type Primitive%20Component%20Object%20Reference) (OtherActor :type Actor%20Object%20Reference) (OtherComp :type Primitive%20Component%20Object%20Reference) (OtherBodyIndex :type Integer))
  (Utilities|Casting|CastToBP_Player OtherActor)
  (Rendering|SetVisibility (Variables|Default|GetHealthWidget) false false))

(event Custom|Attack
  ;[1 1 1] Three in one chance to heavy attack
  (Utilities|FlowControl|DoOnce false :!label _label
    (:Completed
      (switch int (Math|Random|RandomIntegerinRange 0 2)
        (:0
          _)
        (:1
          _)
        (:2
          (bind _returnvalue (Animation|PlayAnimMontage "/Game/Animations/Enemy/AM_Attack_L_02.AM_Attack_L_02" 1.0 "None"))
          (Utilities|FlowControl|Delay _returnvalue)
          (goto _label Reset)))
      (bind _returnvalue_2 (Animation|PlayAnimMontage "/Game/Animations/Enemy/AM_Attack_L_01.AM_Attack_L_01" 1.0 "None"))
      (Utilities|FlowControl|Delay _returnvalue_2)
      (goto _label Reset))))

(event Custom|SetDamageDirection
  (params (DamageDirection :type Vector))
  ;[1 1 1] Calculate which direction the damage came from
  (bind _output_get (Variables|Default|SetDamageDirection (.y (Math|Transform|InverseTransformLocation (Math|Conversions|ToTransform(Vector) DamageDirection) (Transformation|GetWorldLocation (Variables|Character|GetMesh)))))))

(event EventTick
  (params (DeltaSeconds :type Float%20%28single-precision%29))
  (bind _healthwidget (Variables|Default|GetHealthWidget))
  (Transformation|SetWorldRotation _healthwidget (Math|Rotator|FindLookatRotation (Transformation|GetWorldLocation _healthwidget) (Camera|GetCameraLocation (Game|GetPlayerCameraManager 0))) false false))

(event EventBeginPlay
  (bind _output_get (Variables|Default|SetAlive true))
  (AI|Components|Blackboard|SetValueasBool (AI|GetBlackboard (Pawn|GetController)) (Utilities|Name|MakeLiteralName "IsEnemyAlive") _output_get)
  (bind _aswbp_ai_health (Utilities|Casting|CastToWBP_AI_Health (UserInterface|GetUserWidgetObject (Variables|Default|GetHealthWidget))))
  (Variables|Default|SetAs%20WBP%20AI%20Health _aswbp_ai_health))

(event Game|Damage|EventAnyDamage
  (params (Damage :type Float%20%28single-precision%29) (DamageType :type Damage%20Type%20Object%20Reference) (InstigatedBy :type Controller%20Object%20Reference) (DamageCauser :type Actor%20Object%20Reference))
  (bind _damagedirection (Variables|Default|GetDamageDirection))
  (bind _returnvalue (< _damagedirection 0.0))
  ;[1 1 1] Take Damage/Death
  (Utilities|FlowControl|DoOnce false :!label _label
    (:Completed
      (if (> (- (Variables|Default|GetHealth) Damage) 0.0)
        (bind _asbp_player (Utilities|Casting|CastToBP_Player (Game|GetPlayerCharacter 0)))
        (bind _output_get (Variables|Default|SetAs%20BP%20Player _asbp_player))
        (if (and (< (Variables|/Game/Blueprints/Player/BP_Player.BP_Player_C|GetUltimateCharge _output_get) 1e+02) (Variables|/Game/Blueprints/Player/BP_Player.BP_Player_C|GetCanGainUltimate _output_get))
          (bind _output_get_2 (Variables|/Game/Blueprints/Player/BP_Player.BP_Player_C|SetUltimateCharge _output_get (+ (Variables|/Game/Blueprints/Player/BP_Player.BP_Player_C|GetUltimateCharge _output_get) 1e+01))))
        (if (> _output_get_2 1e+02)
          (Variables|/Game/Blueprints/Player/BP_Player.BP_Player_C|SetUltimateCharge _output_get 1e+02))
        (bind _output_get_3 (Variables|Default|SetDamageAmount Damage))
        (bind _output_get_4 (Variables|Default|SetHealth (- (Variables|Default|GetHealth) _output_get_3)))
        (Variables|/Game/UI/Blueprints/WBP_AI_Health.WBP_AI_Health_C|SetHealth (Variables|Default|GetAs%20WBP%20AI%20Health) _output_get_4)
        (if (<= (Variables|Default|GetDamageAmount) 1e+01)
          (if _returnvalue
            (bind _returnvalue_2 (Animation|PlayAnimMontage "/Game/Animations/Enemy/AM_React_Left.AM_React_Left" 1.0 "None"))
            (Utilities|FlowControl|Delay _returnvalue_2)
            (else
              (bind _returnvalue_3 (Animation|PlayAnimMontage "/Game/Animations/Enemy/AM_React_Right.AM_React_Right" 1.0 "None"))
              (Utilities|FlowControl|Delay _returnvalue_3)))
          (elif _returnvalue
            (bind _returnvalue_4 (Animation|PlayAnimMontage "/Game/Animations/Enemy/AM_React_Fwd.AM_React_Fwd" 1.0 "None"))
            (Utilities|FlowControl|Delay _returnvalue_4)
            (else
              (bind _returnvalue_5 (Animation|PlayAnimMontage "/Game/Animations/Enemy/AM_React_Bwd.AM_React_Bwd" 1.0 "None"))
              (Utilities|FlowControl|Delay _returnvalue_5))))
        (Development|PrintString (Utilities|String|ToString(Float) (stale Custom|SetDamageDirection _output_get)))
        (goto _label Reset)
        (else
          (Default|ToggleLockon (Variables|Default|GetAs%20BP%20Player))
          (Rendering|SetVisibility (Variables|Default|GetHealthWidget) false false)
          (Variables|Default|SetAlive false)
          (Collision|SetCollisionEnabled (Variables|Character|GetMesh) "NoCollision")
          (AI|Components|Blackboard|SetValueasBool (AI|GetBlackboard (Pawn|GetController)) (Utilities|Name|MakeLiteralName "IsEnemyAlive") (Variables|Default|GetAlive))
          (bind _returnvalue_6 (Animation|PlayAnimMontage "/Game/Animations/Enemy/AM_Death_01.AM_Death_01" 1.0 "None"))
          (Utilities|FlowControl|Delay (+ _returnvalue_6 5.0))
          (Actor|DestroyActor))))))

(fn ConstructionScript)