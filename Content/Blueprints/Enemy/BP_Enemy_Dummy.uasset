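; Dummy enemy that reacts to hits with montages and feeds the player's overcharge meter, with no health logic.
; AnyDamage passes a DoOnce that resets after the montage-length delay, adding fixed, capped overcharge to BP_Player if it can gain it.
; A macro picks left/right montages for light damage or forward/backward for heavier hits.
; Both pairs use the sign of the hit location's mesh-relative Y, set through a separate SetDamageDirection event.
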(event Custom|SetDamageDirection
  (params (DamageDirection :type Vector))
  ;[1 1 1] Calculate which direction the damage came from
  (Variables|Default|SetDamageDirection (.y (Math|Transform|InverseTransformLocation (Math|Conversions|ToTransform(Vector) DamageDirection) (Transformation|GetWorldLocation (Variables|Character|GetMesh))))))

(event Game|Damage|EventAnyDamage
  (params (Damage :type Float%20%28single-precision%29) (DamageType :type Damage%20Type%20Object%20Reference) (InstigatedBy :type Controller%20Object%20Reference) (DamageCauser :type Actor%20Object%20Reference))
  ;[1 1 1] Take Damage
  (Utilities|FlowControl|DoOnce false :!label _label
    (:Completed
      (Variables|Default|SetDamageAmount Damage)
      (CallFunction|AddPlayerOvercharge 1e+01)
      (Utilities|PlayDamageAnimation
        (:Output
          (goto _label Reset))))))

(fn ConstructionScript)

(fn AddPlayerOvercharge
  (params (Amount :type Float%20%28single-precision%29))
  (bind _asbp_player (Utilities|Casting|CastToBP_Player (Game|GetPlayerCharacter 0)))
  (LocalVariables|SetLoc_Amount Amount)
  (if (and (< (Variables|/Game/Blueprints/Player/BP_Player.BP_Player_C|GetOverchargeMeter _asbp_player) 1e+02) (Variables|/Game/Blueprints/Player/BP_Player.BP_Player_C|GetCanGainOvercharge _asbp_player))
    (Variables|/Game/Blueprints/Player/BP_Player.BP_Player_C|SetOverchargeMeter _asbp_player (Math|Float|Clamp(Float) (+ (Variables|/Game/Blueprints/Player/BP_Player.BP_Player_C|GetOverchargeMeter _asbp_player) (LocalVariables|GetLoc_Amount)) 0.0 1e+02)))
  (return))