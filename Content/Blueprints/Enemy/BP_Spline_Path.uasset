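; BP_Spline_Path is an enemy-related path actor that moves a static mesh along a spline in a repeating loop.
; The SplineSpeed timeline maps its alpha to distance along the spline, sets the mesh's world location, then restarts after a short delay.
; Pause and Continue events stop and resume the timeline.
; A sphere's overlap events track whether a BP_Enemy is inside via OverlappingEnemy, which this graph never reads.
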(event OnComponentBeginOverlap(Sphere)
  (params (OverlappedComponent :type Primitive%20Component%20Object%20Reference) (OtherActor :type Actor%20Object%20Reference) (OtherComp :type Primitive%20Component%20Object%20Reference) (OtherBodyIndex :type Integer) (bFromSweep :type Boolean) (SweepResult :type Hit%20Result%20Structure%20%28by%20ref%29))
  (Utilities|Casting|CastToBP_Enemy OtherActor)
  (Variables|Default|SetOverlappingEnemy true))

(event OnComponentEndOverlap(Sphere)
  (params (OverlappedComponent :type Primitive%20Component%20Object%20Reference) (OtherActor :type Actor%20Object%20Reference) (OtherComp :type Primitive%20Component%20Object%20Reference) (OtherBodyIndex :type Integer))
  (Utilities|Casting|CastToBP_Enemy OtherActor)
  (Variables|Default|SetOverlappingEnemy false))

(event Custom|Continue
  (bind _spline (Variables|Default|GetSpline))
  (bind _newtrack_0 (Timeline|SplineSpeed Play)
    (:Update
      (bind _output_get (Variables|Default|SetLocation (Spline|GetLocationatDistanceAlongSpline _spline (Math|Float|Lerp 0.0 (Spline|GetSplineLength _spline) _newtrack_0) "World")))
      (Transformation|SetWorldLocation (Variables|Default|GetStaticMesh) _output_get false false))
    (:Finished
      (Utilities|FlowControl|Delay 2.0)
      (Timeline|SplineSpeed PlayFromStart))))

(event Custom|Pause
  (bind _spline (Variables|Default|GetSpline))
  (bind _newtrack_0 (Timeline|SplineSpeed Stop)
    (:Update
      (bind _output_get (Variables|Default|SetLocation (Spline|GetLocationatDistanceAlongSpline _spline (Math|Float|Lerp 0.0 (Spline|GetSplineLength _spline) _newtrack_0) "World")))
      (Transformation|SetWorldLocation (Variables|Default|GetStaticMesh) _output_get false false))
    (:Finished
      (Utilities|FlowControl|Delay 2.0)
      (Timeline|SplineSpeed PlayFromStart))))

(event EventBeginPlay
  (bind _spline (Variables|Default|GetSpline))
  (bind _newtrack_0 (Timeline|SplineSpeed PlayFromStart)
    (:Update
      (bind _output_get (Variables|Default|SetLocation (Spline|GetLocationatDistanceAlongSpline _spline (Math|Float|Lerp 0.0 (Spline|GetSplineLength _spline) _newtrack_0) "World")))
      (Transformation|SetWorldLocation (Variables|Default|GetStaticMesh) _output_get false false))
    (:Finished
      (Utilities|FlowControl|Delay 2.0)
      (Timeline|SplineSpeed PlayFromStart))))

(fn ConstructionScript)