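; BP_FightDirector is an early melee fight director that grades listed enemies and picks one to attack.
; On BeginPlay it assigns random grades in a map and attaches a debug widget to each enemy.
; FindHighestGrade, whose comparison seeks lower values despite its name, selects the enemy whose AI controller attacks once before being re-graded.
; The looping one-second TriggerAttack timer only reads the grade values, triggering no attacks.
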(event Custom|TriggerAttack
  (Utilities|Map|Values (Variables|Default|GetEnemyGrading)))

(event EventBeginPlay
  (for _array_element (Variables|Default|GetEnemyList)
    (Utilities|Map|Add (Variables|Default|GetEnemyGrading) _array_element (Math|Random|RandomFloatinRange 1.0 5.0))
    (bind _returnvalue (UserInterface|CreateWidget "/Game/Blueprints/Enemy/WBP_DebugMeleeAI.WBP_DebugMeleeAI_C" 0 _array_element (.Value (Utilities|Map|Find (Variables|Default|GetEnemyGrading) _array_element))))
    (bind _returnvalue_2 (AddComponent|AddWidgetComponent _array_element false))
    (UserInterface|SetWidget _returnvalue_2 _returnvalue))
  (Utilities|Time|SetTimerbyEvent (delegate Custom|TriggerAttack) 1.0 true)
  (bind _loc_highestgradedai1 (CallFunction|FindHighestGrade))
  (bind _asbp_enemy_ai (Utilities|Casting|CastToBP_Enemy_AI (AI|GetAIController _loc_highestgradedai1)))
  (Default|AIAttack _asbp_enemy_ai)
  (Utilities|Map|Add (Variables|Default|GetEnemyGrading) _loc_highestgradedai1 (Math|Random|RandomFloatinRange 1.0 5.0)))

(fn ConstructionScript)

(fn FindHighestGrade
  (bind _keys (Utilities|Map|Keys (Variables|Default|GetEnemyGrading)))
  (for _array_element _keys
    (if (> (LocalVariables|GetLoc_HighestValue) (.Value (Utilities|Map|Find (Variables|Default|GetEnemyGrading) _array_element)))
      (LocalVariables|SetLoc_HighestValue (.Value (Utilities|Map|Find (Variables|Default|GetEnemyGrading) _array_element)))
      (LocalVariables|SetLoc_HighestGradedAI _array_element)))
  (return (LocalVariables|GetLoc_HighestValue) (LocalVariables|GetLoc_HighestGradedAI)))