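; Enemy Blueprint that subtracts incoming damage from Health and plays a directional hit-reaction montage.
; A damage threshold picks light or heavy reactions, and the sign of DamageDirection picks left or right.
; SetDamageDirection derives that value from the local Y of the mesh location relative to the passed-in source.
; A DoOnce gate around montage-length delays limits overlapping hits; no death logic is present despite the graph comment.
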(event Custom|SetDamageDirection
  (params (DamageDirection :type Vector))
  ;[1 1 1] Calculate which direction the damage came from
  (bind _output_get (Variables|Default|SetDamageDirection (.y (Math|Transform|InverseTransformLocation (Math|Conversions|ToTransform(Vector) DamageDirection) (Transformation|GetWorldLocation (Variables|Character|GetMesh)))))))

(event Game|Damage|EventAnyDamage
  (params (Damage :type Float%20%28single-precision%29) (DamageType :type Damage%20Type%20Object%20Reference) (InstigatedBy :type Controller%20Object%20Reference) (DamageCauser :type Actor%20Object%20Reference))
  (bind _damagedirection (Variables|Default|GetDamageDirection))
  (bind _returnvalue (< _damagedirection 0.0))
  ;[1 1 1] Take Damage/Death
  (Utilities|FlowControl|DoOnce false :!label _label
    (:Completed
      (bind _output_get (Variables|Default|SetDamageAmount Damage))
      (Variables|EnemyStats|SetHealth (- (Variables|EnemyStats|GetHealth) _output_get))
      (if (<= (Variables|Default|GetDamageAmount) 1e+01)
        (if _returnvalue
          (bind _returnvalue_2 (Animation|PlayAnimMontage "/Game/Animations/Enemy/AM_Light_Damage_Left.AM_Light_Damage_Left" 1.0 "None"))
          (Utilities|FlowControl|Delay _returnvalue_2)
          (else
            (bind _returnvalue_3 (Animation|PlayAnimMontage "/Game/Animations/Enemy/AM_Light_Damage_Right.AM_Light_Damage_Right" 1.0 "None"))
            (Utilities|FlowControl|Delay _returnvalue_3)))
        (elif _returnvalue
          (bind _returnvalue_4 (Animation|PlayAnimMontage "/Game/Animations/Enemy/AM_Heavy_Damage_Left.AM_Heavy_Damage_Left" 1.0 "None"))
          (Utilities|FlowControl|Delay _returnvalue_4)
          (else
            (bind _returnvalue_5 (Animation|PlayAnimMontage "/Game/Animations/Enemy/AM_Heavy_Damage_Right.AM_Heavy_Damage_Right" 1.0 "None"))
            (Utilities|FlowControl|Delay _returnvalue_5))))
      (Development|PrintString (Utilities|String|ToString(Float) (stale Custom|SetDamageDirection _output_get)))
      (goto _label Reset))))

(fn ConstructionScript)