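; Anim notify state that deals the player's katana light-attack damage to enemies during the attack animation.
; Each tick sphere-traces between the katana start and end sockets on the Camera channel and casts the hit to Patrolling, Dummy or Random enemies.
; A match receives a damage direction (impact point, or zero for Random) and the player's Damage value, with no guard against repeat hits across ticks.
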(fn ReceivedNotifyTick
  (params (MeshComp :type Skeletal%20Mesh%20Component%20Object%20Reference) (Animation :type Anim%20Sequence%20Base%20Object%20Reference) (FrameDeltaTime :type Float%20%28single-precision%29))
  (bind _asbp_player (Utilities|Casting|CastToBP_Player (Game|GetPlayerCharacter MeshComp)))
  (bind _outhit (Collision|SphereTraceByChannel MeshComp (Transformation|GetSocketLocation MeshComp "Katana_Start") (Transformation|GetSocketLocation MeshComp "Katana_End") 1e+01 "TraceTypeQuery2" false 0 "None"))
  ;[1 1 1] Can only damage enemies
  (Utilities|FlowControl|Sequence
    (:then_0
      (bind _asbp_enemy_patrolling (Utilities|Casting|CastToBP_Enemy_Patrolling (.hitactor _outhit)))
      (Default|SetDamageDirection _asbp_enemy_patrolling (.impactpoint _outhit))
      (Game|Damage|ApplyDamage (.hitactor _outhit) (Variables|/Game/Blueprints/Player/BP_Player.BP_Player_C|GetDamage _asbp_player) 0 0))
    (:then_1
      (bind _asbp_enemy_dummy (Utilities|Casting|CastToBP_Enemy_Dummy (.hitactor _outhit)))
      (Default|SetDamageDirection _asbp_enemy_dummy (.impactpoint _outhit))
      (Game|Damage|ApplyDamage (.hitactor _outhit) (Variables|/Game/Blueprints/Player/BP_Player.BP_Player_C|GetDamage _asbp_player) 0 0))
    (:then_2
      (bind _asbp_enemy_random (Utilities|Casting|CastToBP_Enemy_Random (.hitactor _outhit)))
      (Default|SetDamageDirection _asbp_enemy_random "0, 0, 0")
      (Game|Damage|ApplyDamage (.hitactor _outhit) (Variables|/Game/Blueprints/Player/BP_Player.BP_Player_C|GetDamage _asbp_player) 0 0)))
  (return false))