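; BP_Katana is a katana actor that can switch its blade mesh between a standard look and a thermal look.
; On BeginPlay it creates dynamic instances of both materials and enables input from player controller 0.
; The ToggleThermal event, also triggered by the 2 key, swaps the mesh's first material slot between the two instances and flips a Thermal flag.
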(event Custom|ToggleThermal
  (if (Variables|Default|GetThermal)
    (Rendering|Material|SetMaterial (Variables|Default|GetSM_Katana_01) 0 (Variables|Default|GetStandardMaterial))
    (Variables|Default|SetThermal false)
    (else
      (Rendering|Material|SetMaterial (Variables|Default|GetSM_Katana_01) 0 (Variables|Default|GetThermalMaterial))
      (Variables|Default|SetThermal true))))

(event EventBeginPlay
  (bind _returnvalue (Rendering|Material|CreateDynamicMaterialInstance "/Game/Materials/Weapons/M_Katana_Standard.M_Katana_Standard" "None" "None" :!class /Script/Engine.KismetMaterialLibrary))
  (Variables|Default|SetStandardMaterial _returnvalue)
  (bind _returnvalue_2 (Rendering|Material|CreateDynamicMaterialInstance "/Game/Materials/Weapons/M_Katana_Thermal.M_Katana_Thermal" "None" "None" :!class /Script/Engine.KismetMaterialLibrary))
  (Variables|Default|SetThermalMaterial _returnvalue_2)
  (Input|EnableInput (Game|GetPlayerController 0)))

(event Input|KeyboardEvents|2
  (params (Key :type Key%20Structure :default "None"))
  (:Pressed
    (if (Variables|Default|GetThermal)
      (Rendering|Material|SetMaterial (Variables|Default|GetSM_Katana_01) 0 (Variables|Default|GetStandardMaterial))
      (Variables|Default|SetThermal false)
      (else
        (Rendering|Material|SetMaterial (Variables|Default|GetSM_Katana_01) 0 (Variables|Default|GetThermalMaterial))
        (Variables|Default|SetThermal true)))))

(fn ConstructionScript)