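; BP_IKPlayer is a player Blueprint that finds ground contact points under its feet, named for use in foot IK.
; Every tick it sphere-traces downward on the Visibility channel from just above the ball_r and ball_l sockets of its skeletal mesh.
; Each hit's impact point is stored in RightFootLoc or LeftFootLoc, which keep their last value on a miss.
; Both traces draw debug shapes for one frame.
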(event EventTick
  (params (DeltaSeconds :type Float%20%28single-precision%29))
  (bind _skeletalmesh (Variables|Default|GetSkeletalMesh))
  (bind _skeletalmesh_2 (Variables|Default|GetSkeletalMesh))
  (bind _returnvalue (Transformation|GetSocketLocation _skeletalmesh "ball_l"))
  (bind _returnvalue_2 (Transformation|GetSocketLocation _skeletalmesh_2 "ball_r"))
  (bind _returnvalue_3 (+ _returnvalue "0, 0,30.000000"))
  (bind _returnvalue_4 (+ _returnvalue_2 "0, 0,30.000000"))
  (Utilities|FlowControl|Sequence
    (:then_0
      ;[1 1 1] Right Foot Location
      (bind (_outhit _returnvalue_5) (Collision|SphereTraceByChannel _returnvalue_4 (- _returnvalue_4 "0, 0,100.000000") 1.0 "TraceTypeQuery1" false 0 "ForOneFrame"))
      (if _returnvalue_5
        (Variables|Default|SetRightFootLoc (.ImpactPoint (Collision|BreakHitResult _outhit)))))
    (:then_1
      ;[1 1 1] Left Foot Location
      (bind (_outhit_2 _returnvalue_6) (Collision|SphereTraceByChannel _returnvalue_3 (- _returnvalue_3 "0, 0,100.000000") 1.0 "TraceTypeQuery1" false 0 "ForOneFrame"))
      (if _returnvalue_6
        (Variables|Default|SetLeftFootLoc (.ImpactPoint (Collision|BreakHitResult _outhit_2)))))))

(fn ConstructionScript)